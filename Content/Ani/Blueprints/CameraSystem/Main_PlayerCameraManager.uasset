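; Player camera manager that overrides the camera update to follow the possessed pawn.
; On possess, it caches the pawn and hands it and the player controller to the Main_PlayerCameraBehavior anim instance on its CameraBehavior component.
; BlueprintUpdateCamera places the camera at a fixed world-space offset from the pawn, using control rotation and constant FOV.
; The update does not yet read anything from the behavior anim instance.
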(event Custom|OnPossess
  (params (PossessedPawn :type Pawn%20Object%20Reference))
  (bind _output_get (Variables|组件|SetControlledPawn PossessedPawn))
  (bind _asmain_player_camera_behavior (Utilities|Casting|CastToMain_PlayerCameraBehavior (Components|SkeletalMesh|GetAnimInstance (Variables|Default|GetCameraBehavior))))
  (Variables|/Game/Ani/Blueprints/CameraSystem/Main_PlayerCameraBehavior.Main_PlayerCameraBehavior_C|SetPlayerController _asmain_player_camera_behavior (Game|Player|GetOwningPlayerController))
  (Variables|/Game/Ani/Blueprints/CameraSystem/Main_PlayerCameraBehavior.Main_PlayerCameraBehavior_C|SetControlledPawn _asmain_player_camera_behavior _output_get))

(event EventBeginPlay)

(event Collision|EventActorBeginOverlap
  (params (OtherActor :type Actor%20Object%20Reference)))

(event EventTick
  (params (DeltaSeconds :type Float%20%28single-precision%29)))

(fn ConstructionScript)

(fn BlueprintUpdateCamera
  (params (CameraTarget :type Actor%20Object%20Reference))
  (return (+ (Transformation|GetActorLocation (Variables|组件|GetControlledPawn)) "-200.000000,0,150.000000") (Pawn|GetControlRotation (Game|Player|GetOwningPlayerController) :!class /Script/Engine.Controller) 9e+01 true))